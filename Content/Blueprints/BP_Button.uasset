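; BP_Button is an interactable button that triggers a target actor when the player presses E nearby.
; A Sphere overlap with the player pawn toggles input and shows or removes the async-loaded W_Interact prompt widget.
; Pressing E async-loads the soft-referenced InteractableTarget and sends InteractMessage through BPI_Interaction, or prints an error when the reference is invalid.
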(event OnComponentBeginOverlap(Sphere)
  (params (OverlappedComponent :type Primitive%20Component%20Object%20Reference) (OtherActor :type Actor%20Object%20Reference) (OtherComp :type Primitive%20Component%20Object%20Reference) (OtherBodyIndex :type Integer) (bFromSweep :type Boolean) (SweepResult :type Hit%20Result%20Structure%20%28by%20ref%29))
  ;[0 0 0 0.5] Add Press Button Text
  (if (== OtherActor (Game|Player|GetPlayerPawn 0))
    (Input|EnableInput (Game|GetPlayerController 0))
    (bind _class (Utilities|AsyncLoadClassAsset "/Game/Widgets/W_Interact.W_Interact_C")
      (:Completed
        (bind _asuser_widget (Utilities|Casting|CastToUserWidgetClass _class))
        (bind _returnvalue (UserInterface|CreateWidget _asuser_widget))
        (UserInterface|Viewport|AddtoViewport _returnvalue 0)
        (Variables|Default|SetInteractWidget (Utilities|ResolveSoftReference _returnvalue))))))

(event OnComponentEndOverlap(Sphere)
  (params (OverlappedComponent :type Primitive%20Component%20Object%20Reference) (OtherActor :type Actor%20Object%20Reference) (OtherComp :type Primitive%20Component%20Object%20Reference) (OtherBodyIndex :type Integer))
  ;[0 0 0 0.5] Remove Press Button Text
  (if (== OtherActor (Game|Player|GetPlayerPawn 0))
    (Input|DisableInput (Game|GetPlayerController 0))
    (bind _object (Utilities|AsyncLoadAsset (Variables|Default|GetInteractWidget))
      (:Completed
        (bind _asuser_widget (Utilities|Casting|CastToUserWidget _object))
        (Widget|RemovefromParent _asuser_widget)))))

(event Input|KeyboardEvents|E
  (params (Key :type Key%20Structure :default "None"))
  (bind _interactabletarget (Variables|Default|GetInteractableTarget))
  ;[0 0 0 0.5] Press Button
  (:Pressed
    (if (Utilities|IsValidSoftObjectReference _interactabletarget)
      (bind _object (Utilities|AsyncLoadAsset _interactabletarget)
        (:Completed
          (bind _asactor (Utilities|Casting|CastToActor _object))
          (if (Utilities|DoesObjectImplementInterface _asactor "/Game/Blueprints/Interfaces/BPI_Interaction.BPI_Interaction_C")
            (Class|BPIInteraction|Interact(Message) _asactor))))
      (else
        (Development|PrintString "ERROR: No Target set on Button " true true "(R=1.000000,G=0.000000,B=0.000000,A=1.000000)" 5.0)))))

(fn ConstructionScript)