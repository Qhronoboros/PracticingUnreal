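; BP_DodgeGamePlayerPawn is the player pawn for a dodge game, handling health and death.
; On BeginPlay it resets health to maximum, stores its FloatingPawnMovement component and finds the BP_CameraPawn, printing a warning if none exists.
; AnyDamage subtracts clamped damage and, at zero health, fires the OnPlayerDead dispatcher before destroying the actor.
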(event EventBeginPlay
  ;[0.15 0.15 0.15 0.5] Get Necessary Pointers/References
  (Variables|Default|SetHealth (Variables|Default|GetMaxHealth))
  (Variables|Default|Set_pawnMovement (Variables|Default|GetFloatingPawnMovement))
  (bind _returnvalue (Actor|GetActorOfClass "/Game/Blueprints/DodgeGame/BP_CameraPawn.BP_CameraPawn_C"))
  (Variables|Default|Set_cameraPawn _returnvalue)
  (Variables|Default|Get_cameraPawn
    (:then)
    (:else
      (Development|PrintString "CameraPawn Ref is null"))))

(event Game|Damage|EventAnyDamage
  (params (Damage :type Float%20%28single-precision%29) (DamageType :type Damage%20Type%20Object%20Reference) (InstigatedBy :type Controller%20Object%20Reference) (DamageCauser :type Actor%20Object%20Reference))
  ;[0.15 0.15 0.15 0.5] Taking Damage
  (bind _output_get (Variables|Default|SetHealth (Math|Integer|Clamp(Integer) (- (Variables|Default|GetHealth) Damage) 0 (Variables|Default|GetMaxHealth))))
  ;[0.15 0.15 0.15 0.5] Die
  (if (<= _output_get 0)
    (Development|PrintString "Player Dead!")
    (Default|CallOnPlayerDead)
    (Actor|DestroyActor)
    (else
      (Development|PrintString "Player Took Damage!"))))

(fn ConstructionScript)