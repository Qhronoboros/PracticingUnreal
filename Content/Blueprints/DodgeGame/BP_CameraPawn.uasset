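; BP_CameraPawn is the dodge game's camera pawn, which also shows the game-over screen when the player dies.
; On BeginPlay it waits briefly, then calls functions defined outside this graph to receive the viewport corners and center position.
; It then finds BP_DodgeGamePlayerPawn and binds its OnPlayerDead event to create the game-over widget and add it to the viewport.
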(event Custom|CreateGameOverWidget
  ;[0.15 0.15 0.15 0.5] Game Over Widget
  (bind _returnvalue (UserInterface|CreateWidget "/Game/Blueprints/DodgeGame/WB_GameOver.WB_GameOver_C"))
  (bind _output_get (Variables|Default|SetGameOverWidget _returnvalue))
  (UserInterface|Viewport|AddtoViewport _output_get 0))

(event EventBeginPlay
  ;[0.15 0.15 0.15 0.5] Receive Positions
  (Utilities|FlowControl|Delay 0.05)
  (Class|CameraPawn|ReceiveViewportCorners)
  (Class|CameraPawn|ReceiveCenterPosition)
  ;[0.15 0.15 0.15 0.5] PlayerPawn Ref
  (bind _returnvalue (Actor|GetActorOfClass "/Game/Blueprints/DodgeGame/BP_DodgeGamePlayerPawn.BP_DodgeGamePlayerPawn_C"))
  (if (Utilities|IsValid _returnvalue)
    ;[0.15 0.15 0.15 0.5] Game Over Widget
    (EventDispatchers|BindEventtoOnPlayerDead _returnvalue (delegate Custom|CreateGameOverWidget))
    (else
      (Development|PrintString "PlayerPawn Ref is null"))))

(fn ConstructionScript)