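; BPC_PrintAndDestroy is an actor component from an assignment that logs its owner's rotation and lets the player destroy that owner.
; On BeginPlay it enables input on the owning actor for the first player controller.
; Tick prints the owner's rotation every frame, and pressing Space Bar destroys the owning actor.
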(event EventBeginPlay
  ;[0.15 0.15 0.15 0.5] Enable Input
  (Input|EnableInput (Components|GetOwner) (Game|GetPlayerController 0)))

(event EventTick
  (params (DeltaSeconds :type Float%20%28single-precision%29))
  ;[0.15 0.15 0.15 0.5] Print Rotation
  (Development|PrintString (Utilities|String|ToString(Rotator) (Transformation|GetActorRotation (Components|GetOwner)))))

(event Input|KeyboardEvents|SpaceBar
  (params (Key :type Key%20Structure :default "None"))
  ;[0.15 0.15 0.15 0.5] Destroy  Self
  (:Pressed
    (Actor|DestroyActor (Components|GetOwner))))